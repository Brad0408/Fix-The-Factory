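; BP_SlowTrack is a placeable track that pushes actors inside its Box along the direction of its Arrow component, like a conveyor.
; Each Tick, it gets the Box's overlapping actors and offsets each root component by the Arrow's forward vector scaled by Speed and delta time.
; The offset is unswept and applies to every overlapping actor without filtering.
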(event EventBeginPlay
  (|CallParentFunction))

(event Collision|EventActorBeginOverlap
  (params (OtherActor :type Actor%20Object%20Reference))
  (|CallParentFunction OtherActor))

(event EventTick
  (params (DeltaSeconds :type Float%20%28single-precision%29))
  (|CallParentFunction DeltaSeconds)
  (bind _output_get (Variables|Default|SetOverlapping%20Actors (Collision|GetOverlappingActors (Variables|Default|GetBox) 0 :!class /Script/Engine.PrimitiveComponent)))
  (for _array_element _output_get
    (Transformation|AddWorldOffset (Variables|/Script/Engine.Actor|GetRootComponent _array_element) (* (Math|Vector|GetForwardVector (Transformation|GetWorldRotation (Variables|Default|GetArrow))) (* DeltaSeconds (Variables|Default|Getspeed))) false false)))

(fn ConstructionScript
  (|CallParentFunction))