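; BP_InfiniteSpawner is an actor, filed under main menu fakes, that endlessly spawns boxes of a configurable class.
; On BeginPlay it starts a looping timer that spawns the BoxSpawnType class at the Billboard component's location each interval, with no count limit or cleanup.
; It also recolors its Cube purple when the spawn type is the heavy box, as a visual cue.
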(event Custom|SpawnBox
  (Game|SpawnActorfromClass (Variables|Default|GetBox%20Spawn%20Type) (Math|Conversions|ToTransform(Vector) (Transformation|GetWorldLocation (Variables|Default|GetBillboard))) "Undefined" "MultiplyWithRoot" 0 0))

(event Custom|ChangeMaterial
  (if (== (Variables|Default|GetBox%20Spawn%20Type) "/Game/c011185l/BP/BP_BoxHeavyChild.BP_BoxHeavyChild_C")
    (Rendering|Material|SetMaterial (Variables|Default|GetCube) 0 "/Game/c011185l/Materials/FlatColours/M_Purple.M_Purple")))

(event Custom|InitTImers
  (bind _returnvalue (Utilities|Time|SetTimerbyEvent (delegate Custom|SpawnBox) (Variables|Default|GetTime) true))
  (Variables|Default|SetSpawningBoxTimer _returnvalue))

(event EventBeginPlay
  (CallFunction|ChangeMaterial)
  (CallFunction|InitTImers))

(fn ConstructionScript)