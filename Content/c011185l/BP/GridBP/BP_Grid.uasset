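; BP_Grid is a grid manager that spawns a 2D field of BP_IndivdualGridCell actors on BeginPlay and answers nearest-cell queries.
; FillGrid places cells at even gaps on Z=0, offset by half the GridSize extent around world origin rather than the actor's location, and stores them in GridArray.
; Two lookup functions linearly scan that array by distance, returning either the closest cell's location or the cell actor itself.
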(event EventBeginPlay
  (CallFunction|FillGrid))

(fn ConstructionScript)

(fn FillGrid
  (bind _gridgapsize (Variables|Default|GetGridGapSize))
  (bind _gridgapsize_2 (Variables|Default|GetGridGapSize))
  (Utilities|Array|Clear (Variables|Default|GetGridArray))
  (LocalVariables|SetWorldOffset (- (* (* (Variables|Default|GetGridSize) _gridgapsize) 0.5) (* _gridgapsize 0.5)))
  (for _index (range 0 (- (Variables|Default|GetGridX) 1)) ; Loop X
    (for _index_2 (range 0 (- (Variables|Default|GetGridY) 1)) ; Loop Y
      (bind _returnvalue (Game|SpawnActorfromClass "/Game/c011185l/BP/GridBP/BP_IndivdualGridCell.BP_IndivdualGridCell_C" (Math|Transform|MakeTransform (Math|Vector|MakeVector (- (* _index_2 _gridgapsize_2) (LocalVariables|GetWorldOffset)) (- (* _gridgapsize_2 _index) (LocalVariables|GetWorldOffset)) 0.0)) "AlwaysSpawn" "MultiplyWithRoot" 0 0))
      (Utilities|Array|Add (Variables|Default|GetGridArray) _returnvalue))))

(fn GetClosetGridLocation
  (params (InPosition :type Vector))
  (bind _gridarray (Variables|Default|GetGridArray))
  (bind _output (Utilities|Array|Get(acopy) _gridarray))
  (bind _returnvalue (Transformation|GetActorLocation _output))
  (LocalVariables|SetClosetPosition _returnvalue)
  (LocalVariables|SetClosetDistance (Math|Vector|Distance(Vector) InPosition _returnvalue))
  (for _array_element (Variables|Default|GetGridArray)
    (if (< (Math|Vector|Distance(Vector) (Transformation|GetActorLocation _array_element) InPosition) (LocalVariables|GetClosetDistance))
      (LocalVariables|SetClosetPosition (Transformation|GetActorLocation _array_element))
      (LocalVariables|SetClosetDistance (Math|Vector|Distance(Vector) (Transformation|GetActorLocation _array_element) InPosition))))
  (return (LocalVariables|GetClosetPosition)))

(fn GetClosetGridCellLocation
  (params (InPosition :type Vector))
  (LocalVariables|SetClosetDistance (Math|Vector|Distance(Vector) InPosition (Transformation|GetActorLocation (Utilities|Array|Get(acopy) (Variables|Default|GetGridArray)))))
  (for (_array_element _array_index) (Variables|Default|GetGridArray)
    (if (< (Math|Vector|Distance(Vector) (Transformation|GetActorLocation _array_element) InPosition) (LocalVariables|GetClosetDistance))
      (LocalVariables|SetClosetDistance (Math|Vector|Distance(Vector) (Transformation|GetActorLocation _array_element) InPosition))
      (LocalVariables|SetArrayIndex _array_index)))
  (bind _asbp_indivdual_grid_cell (Utilities|Casting|CastToBP_IndivdualGridCell (Utilities|Array|Get(acopy) (Variables|Default|GetGridArray) (LocalVariables|GetArrayIndex))))
  (return _asbp_indivdual_grid_cell))