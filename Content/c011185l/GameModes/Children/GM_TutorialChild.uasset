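; Child game mode for the tutorial level, showing an intro widget before box gameplay and returning to MainMenu when the round ends.
; On BeginPlay it binds to game state changes, floor loss, goal victory and tutorial UI removal, then enters the tutorial text state.
; Removing the intro switches to Gameplaying, which creates gameplay UI and enables the spawner.
; CanEndGame sets GameEnd once enough boxes are secured or failed.
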(event Custom|Init
  (CallFunction|InitGetActorOfClass)
  (CallFunction|BindtoGameState)
  (Default|Init (Variables|Default|GetPC_Ref))
  (CallFunction|RemoveTutUIBind)
  (CallFunction|BindtoFloorCleanup)
  (Default|UpdateState (Variables|Default|GetAs%20GS%20Game%20State) "NewEnumerator0")
  (EventDispatchers|BindEventtoEndGameVictory (Variables|Default|GetGoal_Ref) (delegate Custom|EndGame)))

(event Custom|BindToFloorCleanup
  (EventDispatchers|BindEventtoEndGameLoss (Variables|Default|GetFloor_Ref) (delegate Custom|FloorLoss)))

(event Custom|FloorLoss
  (CallFunction|EndGame))

(event Custom|InitTutorialUI
  ;[1 1 1] Add Tutorial Text To Screen
  (bind _returnvalue (UserInterface|CreateWidget "/Game/c011185l/Widgets/W_TutorialIntro.W_TutorialIntro_C"))
  (bind _output_get (Variables|Default|SetUITutRef _returnvalue))
  (UserInterface|Viewport|AddtoViewport _output_get 0))

(event Custom|BindToGameState
  (bind _output_get (Variables|Default|SetAs%20GS%20Game%20State (.AsGS%20Game%20State (Utilities|Casting|CastToGS_GameState (Game|GetGameState)))))
  (EventDispatchers|BindEventtoGameStateChange _output_get (delegate Custom|ChangeGameState)))

(event Custom|ChangeGameState
  (params (Game%20State :type E_GameState%20Enum :default "NewEnumerator0"))
  (switch Utilities|FlowControl|Switch|SwitchonE_GameState Game%20State
    (:NewEnumerator0
      (Development|PrintString "PreGame")
      (CallFunction|InitTutorialUI))
    (:NewEnumerator1
      (Development|PrintString "GamePlay")
      (CallFunction|InitGamePlayUI)
      (Default|CallEnableSpawner))
    (:NewEnumerator2
      (Development|PrintString "Game E d")
      (CallFunction|EndGame))))

(event Custom|EndGame
  (Game|OpenLevel(byName) "MainMenu"))

(event Custom|RemoveTutUIBind
  ;[1 1 1] Remove Tutorial Text and Change to Gameplay
  (EventDispatchers|BindEventtoRemoveTutUI (delegate Custom|ProperTutRemove)))

(event Custom|ProperTutRemove
  ;[1 1 1] Remove Tutorial Text and Change to Gameplay
  (Widget|RemovefromParent (Variables|Default|GetUITutRef))
  (Default|UpdateState (Variables|Default|GetAs%20GS%20Game%20State) "NewEnumerator1"))

(event EventTick
  (params (DeltaSeconds :type Float%20%28single-precision%29))
  (|CallParentFunction DeltaSeconds))

(event EventBeginPlay
  (|CallParentFunction)
  (bind _returnvalue (Actor|GetActorOfClass "/Game/c011185l/PlayerControllers/PC_Tutorial.PC_Tutorial_C"))
  (bind _output_get (Variables|Default|SetPC_Ref _returnvalue))
  (Input|SetInputModeGameOnly _output_get false)
  (Development|PrintString "GM_Tutorial (CHild)")
  (CallFunction|Init))

(fn ConstructionScript
  (|CallParentFunction))

(fn CanEndGame
  (if (or (Variables|Default|GetEnoughBoxesSecured) (Variables|Default|GetEnoughBoxesFailed))
    (Default|UpdateState (Variables|Default|GetAs%20GS%20Game%20State) "NewEnumerator2")))