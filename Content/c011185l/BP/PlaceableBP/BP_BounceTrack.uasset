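; BP_BounceTrack is a placeable bounce pad that launches the first-person player and physics boxes.
; Any overlap with its Box trigger plays the Bouncer sound at the actor.
; The player character receives a fixed upward LaunchCharacter boost, added to its current velocity.
; BP_BoxNormalChild boxes instead get a mass-independent impulse on their Cube along the Arrow's forward direction, scaled by LaunchSpeed.
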(event OnComponentBeginOverlap(Box)
  (params (OverlappedComponent :type Primitive%20Component%20Object%20Reference) (OtherActor :type Actor%20Object%20Reference) (OtherComp :type Primitive%20Component%20Object%20Reference) (OtherBodyIndex :type Integer) (bFromSweep :type Boolean) (SweepResult :type Hit%20Result%20Structure%20%28by%20ref%29))
  (Audio|SpawnSoundatLocation "/Game/c011185l/Audio/SFX/bouncer.bouncer" (Transformation|GetActorLocation) "0, 0, 0" 1.0 1.0 0.0 "/Game/c011185l/Audio/ATT_Bouncer.ATT_Bouncer" 0)
  (bind _asbp_first_person_character (Utilities|Casting|CastToBP_FirstPersonCharacter OtherActor)
    (:then
      (Character|LaunchCharacter _asbp_first_person_character "0.000000,0.000000,750.000000" false false))
    (:CastFailed
      (bind _asbp_box_normal_child (Utilities|Casting|CastToBP_BoxNormalChild OtherActor))
      (Physics|AddImpulse (Variables|/Game/c011185l/BP/BP_Box.BP_Box_C|GetCube _asbp_box_normal_child) (* (Math|Vector|GetForwardVector (Transformation|GetWorldRotation (Variables|Default|GetArrow))) (Variables|Default|GetLaunchSpeed)) "None" true))))

(event Collision|EventActorBeginOverlap
  (params (OtherActor :type Actor%20Object%20Reference))
  (|CallParentFunction OtherActor) ; This node is disabled and will not be called.\nDrag off pins to build functionality.
)

(fn ConstructionScript
  (|CallParentFunction))