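; Main menu player controller that puts the main menu widget on screen with a visible cursor and game-and-UI input.
; On BeginPlay it caches the GI_Data game instance, sets a camera type enum and pre-creates the level and settings widgets as stored references.
; A debug M key unlocks all levels by flagging the tutorial and three levels complete in the game instance.
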(event EventBeginPlay
  (Variables|Default|SetGameInstance (.AsGI%20Data (Utilities|Casting|CastToGI_Data (Game|GetGameInstance))))
  ;[1 1 1] Set UI only and add main menu widget to screen
  (Variables|Default|SetbShowMouseCursor true)
  (bind _returnvalue (UserInterface|CreateWidget "/Game/c011185l/Widgets/W_NewMainMenu.W_NewMainMenu_C" self))
  (bind _output_get (Variables|Default|SetNewMainMenuRef _returnvalue))
  (UserInterface|Viewport|AddtoViewport _output_get 0)
  (Input|SetInputModeGameandUI self _output_get "DoNotLock" true false)
  ;[1 1 1] Set the camera type and also create references to the other UI elements
  (Variables|Default|SetCameraEnum "NewEnumerator0")
  (bind _returnvalue_2 (UserInterface|CreateWidget "/Game/c011185l/Widgets/W_Levels.W_Levels_C"))
  (Variables|Default|SetLevelWidgetRef _returnvalue_2)
  (bind _returnvalue_3 (UserInterface|CreateWidget "/Game/c011185l/Widgets/W_SettingsMenu.W_SettingsMenu_C"))
  (Variables|Default|SetSettingsRef _returnvalue_3))

(event Input|KeyboardEvents|M
  (params (Key :type Key%20Structure :default "None"))
  (bind _gameinstance (Variables|Default|GetGameInstance))
  ;[1 1 1] debug option - unlock all levels
  (:Pressed
    (Variables|/Game/c011185l/GI_Data.GI_Data_C|SetTutorialComplete _gameinstance true)
    (Variables|/Game/c011185l/GI_Data.GI_Data_C|SetLevel1Complete _gameinstance true)
    (Variables|/Game/c011185l/GI_Data.GI_Data_C|SetLevel2Complete _gameinstance true)
    (Variables|/Game/c011185l/GI_Data.GI_Data_C|SetLevel3Complete _gameinstance true)))

(fn ConstructionScript)

(fn GetTrackCount
  (return ""))