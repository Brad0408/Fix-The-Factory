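; Player controller for local multiplayer that holds each player's data, including team ID.
; SetPlayerData and SetTeam write the PlayerData struct, and GetPlayerData and GetTeam read it back.
; The M key removes all players and opens the main menu.
; Debug numpad keys switch input between players 1 and 2 by reassigning controller ID 0, while matching logic for players 3 and 4 is left unwired.
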(event EventBeginPlay
  (Development|PrintString "PC_Multiplayer Running" true true "(R=0.000000,G=0.660000,B=1.000000,A=1.000000)" 1e+01))

(event EventSetTeam
  (params (TeamID :type E_Teams%20Enum :default "NewEnumerator0"))
  (Utilities|Struct|SetmembersinS_PlayerData (Variables|Default|GetPlayerData) TeamID))

(event EventSetPlayerData
  (params (Player%20Data :type S%20Player%20Data%20Structure))
  (Variables|Default|SetPlayerData Player%20Data))

(event Input|KeyboardEvents|DebugKeyNumPadZero
  (params (Key :type Key%20Structure :default "None") (ActionValue :type Input%20Action%20Value%20Structure))
  ;[1 1 1] Possess Other Players
  (:Pressed
    (Development|PrintString "Possess Player 1")
    (Class|GameplayStatics|SetPlayerControllerID (Game|GetPlayerController 0))))

(event Input|KeyboardEvents|DebugKeyNumPadOne
  (params (Key :type Key%20Structure :default "None") (ActionValue :type Input%20Action%20Value%20Structure))
  ;[1 1 1] Possess Other Players
  (:Pressed
    (Development|PrintString "Possess Player 2")
    (Class|GameplayStatics|SetPlayerControllerID (Game|GetPlayerController 1))))

(event Input|KeyboardEvents|DebugKeyNumPadTwo
  (params (Key :type Key%20Structure :default "None") (ActionValue :type Input%20Action%20Value%20Structure))
  ;[1 1 1] Possess Other Players
)

(event Input|KeyboardEvents|DebugKeyNumPadThree
  (params (Key :type Key%20Structure :default "None") (ActionValue :type Input%20Action%20Value%20Structure))
  ;[1 1 1] Possess Other Players
)

(event Input|KeyboardEvents|M
  (params (Key :type Key%20Structure :default "None"))
  (:Pressed
    (CallFunction|RemoveAllPlayers)
    (Game|OpenLevel(byName) "MainMenu")))

(fn ConstructionScript)

(fn GetPlayerData
  (return (Variables|Default|GetPlayerData)))

(fn GetTeam
  (return (.TeamID (Utilities|Struct|BreakS_PlayerData (Variables|Default|GetPlayerData)))))