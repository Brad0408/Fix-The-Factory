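; Tutorial player controller that switches player movement and cursor visibility to match the current game state.
; Init, which is not called within this asset, binds GameStateChanged to GS_GameState's state-change event.
; The text box state disables movement and shows the cursor, while Gameplaying and Game End both restore walking and hide it.
; The M key opens the MainMenu level, and each state change prints a debug string.
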(event Custom|Init
  (EventDispatchers|BindEventtoGameStateChange (.AsGS%20Game%20State (Utilities|Casting|CastToGS_GameState (Game|GetGameState))) (delegate Custom|GameStateChanged)))

(event Custom|GameStateChanged
  (params (Game%20State :type E_GameState%20Enum :default "NewEnumerator0"))
  (bind _returnvalue (Game|GetPlayerCharacter 0))
  (bind _returnvalue_2 (Game|GetPlayerController 0))
  (bind _charactermovement (Variables|/Script/Engine.Character|GetCharacterMovement _returnvalue))
  (Development|PrintString "CHANGES")
  (switch Utilities|FlowControl|Switch|SwitchonE_GameState Game%20State
    (:NewEnumerator0
      (Pawn|Components|CharacterMovement|DisableMovement _charactermovement) ; Needed so if you press 'Tab' while moving you still stop
      (Variables|/Script/Engine.PlayerController|SetbShowMouseCursor _returnvalue_2 true))
    (:NewEnumerator1
      (Pawn|Components|CharacterMovement|SetMovementMode _charactermovement "MOVE_Walking" 0 :!label _label)
      (Variables|/Script/Engine.PlayerController|SetbShowMouseCursor _returnvalue_2 false))
    (:NewEnumerator2
      (goto _label))))

(event EventBeginPlay)

(event Input|KeyboardEvents|M
  (params (Key :type Key%20Structure :default "None"))
  (:Pressed
    (Game|OpenLevel(byName) "MainMenu")))

(fn ConstructionScript)