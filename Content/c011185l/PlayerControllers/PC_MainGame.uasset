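; PC_MainGame is the in-game player controller that provides keyboard shortcuts for changing levels.
; Pressing P reads the current level name and reopens it if it matches one of three numbered levels, acting as a restart through a chain of name comparisons.
; Pressing M opens the main menu, and BeginPlay prints the controller's name as a debug string.
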(event EventBeginPlay
  (Development|PrintString "PC_MainGame"))

(event Input|KeyboardEvents|M
  (params (Key :type Key%20Structure :default "None"))
  (:Pressed
    (Game|OpenLevel(byName) "MainMenu")))

(event Input|KeyboardEvents|P
  (params (Key :type Key%20Structure :default "None"))
  (:Pressed
    (bind _returnvalue (Game|GetCurrentLevelName true))
    (if (== (Utilities|String|StringToName _returnvalue) "Level_1")
      ;[1 1 1] Lvl1
      (Game|OpenLevel(byName) "Level_1")
      (elif (== (Utilities|String|StringToName _returnvalue) "Level_2")
        ;[1 1 1] Lvl2
        (Game|OpenLevel(byName) "Level_2")
        (elif (== (Utilities|String|StringToName _returnvalue) "Level_3")
          (Game|OpenLevel(byName) "Level_3"))))))

(fn ConstructionScript)