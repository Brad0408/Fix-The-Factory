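; BP_ConvTest is a test conveyor actor in the placeable Blueprints' old tests folder that pushes whatever overlaps its box.
; Every Tick, it offsets the root component of each actor overlapping the Box along the Arrow's forward vector, scaled by Speed and delta time.
; Movement is a direct world offset without sweep, so it ignores blocking collision.
; A leftover overlap debug print never runs.
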(event EventTick
  (params (DeltaSeconds :type Float%20%28single-precision%29))
  (for _array_element (Collision|GetOverlappingActors (Variables|Default|GetBox) 0 :!class /Script/Engine.PrimitiveComponent)
    (Transformation|AddWorldOffset (Variables|/Script/Engine.Actor|GetRootComponent _array_element) (* (Math|Vector|GetForwardVector (Transformation|GetWorldRotation (Variables|Default|GetArrow))) (* DeltaSeconds (Variables|Default|Getspeed))) false false)))

(fn ConstructionScript)