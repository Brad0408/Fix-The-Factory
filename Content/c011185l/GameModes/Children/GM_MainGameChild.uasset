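; GM_MainGameChild is a child game mode that starts up a main-game session and keeps the top-right count display updated.
; On BeginPlay it sets game-only input on PC_MainGame, then runs Init to set up actor references, gameplay UI, floor-cleanup binding and end-game victory.
; It binds the first-person reference's top-right update event to forward a track type to the count update.
; After a short delay it enables the spawner.
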(event Custom|Init
  (CallFunction|InitGetActorOfClass)
  (CallFunction|InitGamePlayUI)
  (CallFunction|BindtoFloorCleanup)
  (CallFunction|EndGameVictory))

(event Custom|Updaet
  (params (TrackTYpe :type E_PlacedAssetType%20Enum :default "NewEnumerator0"))
  (CallFunction|UpdateTopRightCount TrackTYpe))

(event EventBeginPlay
  (|CallParentFunction)
  (Development|PrintString "GM_MainGame Running")
  (bind _returnvalue (Actor|GetActorOfClass "/Game/c011185l/PlayerControllers/PC_MainGame.PC_MainGame_C"))
  (bind _output_get (Variables|Default|SetPC_Ref _returnvalue))
  (Input|SetInputModeGameOnly _output_get false)
  (CallFunction|Init)
  (EventDispatchers|BindEventtoUpdateTopRight (Variables|Default|GetFirstPersonRef) (delegate Custom|Updaet))
  (Utilities|FlowControl|Delay 3.0)
  (Default|CallEnableSpawner))

(event EventTick
  (params (DeltaSeconds :type Float%20%28single-precision%29))
  (|CallParentFunction DeltaSeconds))

(fn ConstructionScript
  (|CallParentFunction))