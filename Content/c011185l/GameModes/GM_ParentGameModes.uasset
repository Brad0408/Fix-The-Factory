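; Parent game mode for a conveyor-track placement game, providing shared setup and HUD events.
; Events create the W_MainGameplay widget and cache references to the BP_BoxGoal actors and BP_FloorCleanup.
; FireSetCount matches the player's placed track type to its AssetMenu count and sends it to the gameplay UI.
; The lookup that sets the first-person character reference is unconnected in this graph.
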(event Custom|InitGamePlayUI
  (bind _returnvalue (UserInterface|CreateWidget "/Game/c011185l/Widgets/W_MainGameplay.W_MainGameplay_C"))
  (bind _output_get (Variables|Default|SetUIgameplay_Ref _returnvalue))
  (UserInterface|Viewport|AddtoViewport _output_get 0))

(event Custom|FireSetCount
  (bind _firstpersonref (Variables|Default|GetFirstPersonRef))
  (bind _uigameplay_ref (Variables|Default|GetUIgameplay_Ref))
  (bind _assetmenu (Variables|/Game/FirstPerson/Blueprints/BP_FirstPersonCharacter.BP_FirstPersonCharacter_C|GetAssetMenu _firstpersonref))
  (switch Utilities|FlowControl|Switch|SwitchonE_PlacedAssetType (Variables|/Game/FirstPerson/Blueprints/BP_FirstPersonCharacter.BP_FirstPersonCharacter_C|GetPlacedObjectType _firstpersonref)
    (:NewEnumerator0
      (Default|SetTrackCountforGameplay _uigameplay_ref 5))
    (:NewEnumerator1
      (Default|SetTrackCountforGameplay _uigameplay_ref (Variables|/Game/c011185l/Widgets/W_AssetMenu.W_AssetMenu_C|GetSimple _assetmenu)))
    (:NewEnumerator2
      (Default|SetTrackCountforGameplay _uigameplay_ref (Variables|/Game/c011185l/Widgets/W_AssetMenu.W_AssetMenu_C|GetBouncer _assetmenu)))
    (:NewEnumerator3
      (Default|SetTrackCountforGameplay _uigameplay_ref (Variables|/Game/c011185l/Widgets/W_AssetMenu.W_AssetMenu_C|GetFast _assetmenu)))
    (:NewEnumerator4
      (Default|SetTrackCountforGameplay _uigameplay_ref (Variables|/Game/c011185l/Widgets/W_AssetMenu.W_AssetMenu_C|GetSlow _assetmenu)))))

(event Custom|InitGetActorOfClass
  (bind _outactors (Actor|GetAllActorsOfClass "/Game/c011185l/BP/BP_BoxGoal.BP_BoxGoal_C"))
  (Variables|Default|SetGoal_Ref _outactors)
  (bind _returnvalue (Actor|GetActorOfClass "/Game/c011185l/BP/BP_FloorCleanup.BP_FloorCleanup_C"))
  (Variables|Default|SetFloor_Ref _returnvalue))

(fn ConstructionScript)