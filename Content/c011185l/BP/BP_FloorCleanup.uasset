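; BP_FloorCleanup is a floor trigger that catches dropped boxes and ends the game in a loss when too many fall.
; When a BP_Box overlaps its Box component, it increments the dropped count, updates the gameplay UI through the cached GM_ParentGameModes reference, destroys the box and plays a poof sound.
; LossCheck then compares the count to AMOUNTTOFAIL, calls the loss end-game event and pauses the game.
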(event OnComponentBeginOverlap(Box)
  (params (OverlappedComponent :type Primitive%20Component%20Object%20Reference) (OtherActor :type Actor%20Object%20Reference) (OtherComp :type Primitive%20Component%20Object%20Reference) (OtherBodyIndex :type Integer) (bFromSweep :type Boolean) (SweepResult :type Hit%20Result%20Structure%20%28by%20ref%29))
  ;[1 1 1] If a box overlaps, destroy and add one to dropped counter
  (bind _asbp_box (Utilities|Casting|CastToBP_Box OtherActor))
  (bind _result (Math|Integer|IncrementInt (Variables|Default|GetDroppedCount))
    (:%20%20
      (Default|IncreaseDroppedBoxes (Variables|/Game/c011185l/GameModes/GM_ParentGameModes.GM_ParentGameModes_C|GetUIgameplay_Ref (stale EventBeginPlay _output_get)) _result)
      (Actor|DestroyActor _asbp_box)
      (Audio|PlaySoundatLocation "/Game/c011185l/Audio/SFX/boxpoof.boxpoof" "0, 0, 0" "0, 0, 0" 1.0 1.0 0.0 0 0 0 0)
      (CallFunction|LossCheck))))

(event Custom|LossCheck
  ;[1 1 1] If 3 dropped , end game
  (if (>= (Variables|Default|GetDroppedCount) (Variables|Default|GetAMOUNT%20TO%20FAIL))
    (Default|CallEndGameLoss)
    (Game|SetGamePaused true)))

(event EventBeginPlay
  ;[1 1 1] If a box overlaps, destroy and add one to dropped counter
  (bind _returnvalue (Actor|GetActorOfClass "/Game/c011185l/GameModes/GM_ParentGameModes.GM_ParentGameModes_C"))
  (bind _output_get (Variables|Default|SetBassGM_Ref _returnvalue)))

(fn ConstructionScript)