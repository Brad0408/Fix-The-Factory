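; Child game mode that sets up a local two-player team match, one player on Team A and one on Team B.
; On BeginPlay it writes both players' data to the GI_Data game instance, then replaces the default player with controllers created from that data and sorts them into team lists.
; PostLogin tracks controllers; each then possesses its pawn class, spawned at a random team-matched BP_NewPlayerStart.
; SetUpControllers, an uncalled count-based variant, alternates teams via FlipFlop.
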(event Custom|Init
  (CallFunction|SettingPlayerData)
  (CallFunction|SetUpControllersGI)
  (CallFunction|SpawnCharacters))

(event Custom|SettingPlayerData
  (bind _gameinstance_0 (Variables|Default|GetGameInstance_0))
  (Utilities|Struct|SetmembersinS_PlayerData (Variables|/Game/c011185l/GIAndMisc/GI_Data.GI_Data_C|GetPlayer0_Data _gameinstance_0) 0 "/Game/c011185l/BP/MultiPlayer/BP_FirstPersonPlayer1.BP_FirstPersonPlayer1_C" "NewEnumerator1" true)
  (Utilities|Struct|SetmembersinS_PlayerData (Variables|/Game/c011185l/GIAndMisc/GI_Data.GI_Data_C|GetPlayer1_Data _gameinstance_0) 1 "/Game/c011185l/BP/MultiPlayer/BP_FirstPersonPlayer2.BP_FirstPersonPlayer2_C" "NewEnumerator2" true))

(event EventBeginPlay
  (|CallParentFunction)
  (Variables|Default|SetGameInstance_0 (.AsGI%20Data (Utilities|Casting|CastToGI_Data (Game|GetGameInstance))))
  (for _array_element (Variables|Default|GetAllGamePlayControllers)
    _)
  (Input|SetInputModeGameOnly _array_element false)
  (CallFunction|Init))

(event EventOnLogout
  (params (ExitingController :type Controller%20Object%20Reference))
  (bind _aspc_multi_player (Utilities|Casting|CastToPC_MultiPlayer ExitingController))
  (Utilities|Array|RemoveItem (Variables|Default|GetAllGamePlayControllers) _aspc_multi_player))

(event EventPostLogin
  (params (NewPlayer :type Player%20Controller%20Object%20Reference))
  (bind _aspc_multi_player (Utilities|Casting|CastToPC_MultiPlayer NewPlayer))
  (Utilities|Array|Add (Variables|Default|GetAllGamePlayControllers) _aspc_multi_player))

(fn ConstructionScript
  (|CallParentFunction))

(fn SetUpControllers
  (params (Number%20of%20players :type Integer))
  (Class|GameplayStatics|RemovePlayer (Game|GetPlayerController 0) true)
  (for _index (range 0 (- Number%20of%20players 1))
    (bind _returnvalue (Class|GameplayStatics|CreatePlayer _index))
    (Utilities|FlowControl|FlipFlop
      (:A
        (Class|BPITeams|SetTeam(Message) _returnvalue "NewEnumerator1"))
      (:B
        (Class|BPITeams|SetTeam(Message) _returnvalue "NewEnumerator2")))
    (CallFunction|AddtoTeamList (.AsPC%20Multi%20Player (Utilities|Casting|CastToPC_MultiPlayer _returnvalue)))))

(fn SpawnCharacters
  (for _array_element (Variables|Default|GetAllGamePlayControllers)
    (bind _playerdata (Class|BPITeams|GetPlayerData(Message) _array_element))
    (bind _returnvalue (Game|SpawnActorfromClass (.PlayerClass (Utilities|Struct|BreakS_PlayerData _playerdata)) (Transformation|GetActorTransform (CallFunction|SelectPlayerStart (.TeamID (Utilities|Struct|BreakS_PlayerData _playerdata)))) "AdjustIfPossibleButAlwaysSpawn" "MultiplyWithRoot" 0 0 0))
    (Pawn|Possess _array_element (.AsPawn (Utilities|Casting|CastToPawn _returnvalue)))))

(fn SelectPlayerStart
  (params (TeamID :type E_Teams%20Enum :default "NewEnumerator0"))
  (bind _outactors (Actor|GetAllActorsOfClass "/Game/c011185l/BP/MultiPlayer/BP_NewPlayerStart.BP_NewPlayerStart_C"))
  (for _array_element _outactors
    (bind _teamid (Class|BPITeams|GetTeam(Message) _array_element))
    (if (Utilities|Enum|Equal(Enum) _teamid TeamID)
      (Utilities|Array|Add (LocalVariables|GetL_SpawnPointActors) _array_element)))
  (if (!= (Utilities|Array|Length (LocalVariables|GetL_SpawnPointActors)) 0)
    (return (.OutItem (Utilities|Array|Random (LocalVariables|GetL_SpawnPointActors))))
    (else
      (bind _returnvalue (Actor|GetActorOfClass "/Game/c011185l/BP/MultiPlayer/BP_NewPlayerStart.BP_NewPlayerStart_C"))
      (return _returnvalue))))

(fn AddtoTeamList
  (params (GP%20Controller :type PC%20Multi%20Player%20Object%20Reference))
  (bind _teamid (Class|BPITeams|GetTeam(Message) GP%20Controller))
  (switch Utilities|FlowControl|Switch|SwitchonE_Teams _teamid
    (:NewEnumerator1
      (Utilities|Array|Add (Variables|Default|GetTeamAPlayers) GP%20Controller))
    (:NewEnumerator2
      (Utilities|Array|Add (Variables|Default|GetTeamBPlayers) GP%20Controller))))

(fn SetUpControllersGI
  (bind _gameinstance_0 (Variables|Default|GetGameInstance_0))
  (Class|GameplayStatics|RemovePlayer (Game|GetPlayerController 0) true)
  (for _index (range 0 2)
    (if (.isActive (Utilities|Struct|BreakS_PlayerData (Utilities|Select :Index _index :Option%200 (Variables|/Game/c011185l/GIAndMisc/GI_Data.GI_Data_C|GetPlayer0_Data _gameinstance_0) :Option%201 (Variables|/Game/c011185l/GIAndMisc/GI_Data.GI_Data_C|GetPlayer1_Data _gameinstance_0))))
      (bind _returnvalue (Class|GameplayStatics|CreatePlayer (.PlayerID (Utilities|Struct|BreakS_PlayerData (Utilities|Select :Index _index :Option%200 (Variables|/Game/c011185l/GIAndMisc/GI_Data.GI_Data_C|GetPlayer0_Data _gameinstance_0) :Option%201 (Variables|/Game/c011185l/GIAndMisc/GI_Data.GI_Data_C|GetPlayer1_Data _gameinstance_0))))))
      (Class|BPITeams|SetPlayerData(Message) _returnvalue (Utilities|Select :Index _index :Option%200 (Variables|/Game/c011185l/GIAndMisc/GI_Data.GI_Data_C|GetPlayer0_Data _gameinstance_0) :Option%201 (Variables|/Game/c011185l/GIAndMisc/GI_Data.GI_Data_C|GetPlayer1_Data _gameinstance_0)))
      (CallFunction|AddtoTeamList (.AsPC%20Multi%20Player (Utilities|Casting|CastToPC_MultiPlayer _returnvalue))))))