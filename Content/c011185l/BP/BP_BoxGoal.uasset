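; BP_BoxGoal is a goal actor that scores BP_Box actors entering its trigger and calls victory for the level.
; Each overlap raises the score, updates the gameplay UI through the game mode, runs the win check and destroys the box.
; Victory requires at least 70% of the spawner's boxes scored, with scored plus floor-dropped equalling the spawn total.
; That check runs only when a box scores.
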(event OnComponentBeginOverlap(Box)
  (params (OverlappedComponent :type Primitive%20Component%20Object%20Reference) (OtherActor :type Actor%20Object%20Reference) (OtherComp :type Primitive%20Component%20Object%20Reference) (OtherBodyIndex :type Integer) (bFromSweep :type Boolean) (SweepResult :type Hit%20Result%20Structure%20%28by%20ref%29))
  (bind _asbp_box (Utilities|Casting|CastToBP_Box OtherActor))
  (Math|Integer|IncrementInt (Variables|Default|GetScore)
    (:%20%20
      (Default|IncreaseScoredUI (Variables|/Game/c011185l/GameModes/GM_ParentGameModes.GM_ParentGameModes_C|GetUIgameplay_Ref (stale EventBeginPlay _output_get)) (Variables|Default|GetScore))
      (CallFunction|EndCheck)
      (Actor|DestroyActor _asbp_box)
      (Default|Cleared (Variables|/Game/c011185l/GameModes/GM_ParentGameModes.GM_ParentGameModes_C|GetUIgameplay_Ref (stale EventBeginPlay _output_get))))))

(event Custom|End%20Check
  (if (>= (Variables|Default|GetScore) (stale EventBeginPlay _output_get_2))
    (if (== (+ (Variables|Default|GetScore) (Variables|/Game/c011185l/BP/BP_FloorCleanup.BP_FloorCleanup_C|GetDroppedCount (Variables|/Game/c011185l/GameModes/GM_ParentGameModes.GM_ParentGameModes_C|GetFloor_Ref (stale EventBeginPlay _output_get)))) (Variables|/Game/c011185l/BP/BP_BoxSpawner.BP_BoxSpawner_C|GetBoxesToSpawn (Variables|Default|GetSpawnerRef)))
      (Development|PrintString "YOU WIN" true true "(R=0.000000,G=1.000000,B=0.161790,A=1.000000)" 1e+01)
      (Default|CallEndGameVictory))))

(event EventBeginPlay
  (bind _returnvalue (Actor|GetActorOfClass "/Game/c011185l/BP/BP_BoxSpawner.BP_BoxSpawner_C"))
  (Variables|Default|SetSpawnerRef _returnvalue)
  (bind _returnvalue_2 (Actor|GetActorOfClass "/Game/c011185l/GameModes/GM_ParentGameModes.GM_ParentGameModes_C"))
  (bind _output_get (Variables|Default|SetBassGM_Ref _returnvalue_2))
  (bind _output_get_2 (Variables|Default|SetPercentageOfBoxes (* (Variables|/Game/c011185l/BP/BP_BoxSpawner.BP_BoxSpawner_C|GetBoxesToSpawn (Variables|Default|GetSpawnerRef)) 0.7)))
  (Development|PrintString (Utilities|String|ToString(Integer) _output_get_2)))

(fn ConstructionScript)