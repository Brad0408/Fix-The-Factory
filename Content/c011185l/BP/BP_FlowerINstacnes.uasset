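; BP_FlowerINstacnes is a flower scatter actor that fills a configurable Length, Width and Height grid with instanced static meshes.
; The Construction Script loops over the grid, using a FlipFlop to alternate instances between two InstancedStaticMesh components.
; Each grid index is multiplied by a random spacing per axis for jittered placement, with random rotation up to RotationVariacne and a fixed scale.
; The event graph holds no gameplay logic.
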(event EventBeginPlay)

(event Collision|EventActorBeginOverlap
  (params (OtherActor :type Actor%20Object%20Reference)))

(event EventTick
  (params (DeltaSeconds :type Float%20%28single-precision%29)))

(fn ConstructionScript
  (bind _rotationvariacne (Variables|Default|GetRotationVariacne))
  (bind _spacing (Variables|Default|GetSpacing))
  (bind _returnvalue (Math|Random|RandomFloatinRange 0.0 (.yaw _rotationvariacne)))
  (bind _returnvalue_2 (Math|Random|RandomFloatinRange 0.0 (.roll _rotationvariacne)))
  (bind _returnvalue_3 (Math|Random|RandomFloatinRange 0.0 (.pitch _rotationvariacne)))
  (bind _returnvalue_4 (Math|Rotator|MakeRotator _returnvalue_2 _returnvalue_3 _returnvalue))
  (for _index (range 0 (- (Variables|Default|GetHeight) 1))
    (for _index_2 (range 0 (- (Variables|Default|GetWidth) 1))
      (for _index_3 (range 0 (- (Variables|Default|GetLength) 1))
        (Utilities|FlowControl|FlipFlop
          (:A
            (Components|InstancedStaticMesh|AddInstance (Variables|Default|GetInstancedStaticMesh) (Math|Transform|MakeTransform (* (Math|Vector|MakeVector (Math|Conversions|ToFloat(Integer) _index_3) (Math|Conversions|ToFloat(Integer) _index_2) (Math|Conversions|ToFloat(Integer) _index)) (Math|Vector|MakeVector (Math|Random|RandomFloatinRange 0.0 (.x _spacing)) (Math|Random|RandomFloatinRange 0.0 (.y _spacing)) (Math|Random|RandomFloatinRange 0.0 (.z _spacing)))) _returnvalue_4 "2.000000,2.000000,2.000000") false))
          (:B
            (Components|InstancedStaticMesh|AddInstance (Variables|Default|GetInstancedStaticMesh1) (Math|Transform|MakeTransform (* (Math|Vector|MakeVector (Math|Conversions|ToFloat(Integer) _index_3) (Math|Conversions|ToFloat(Integer) _index_2) (Math|Conversions|ToFloat(Integer) _index)) (Math|Vector|MakeVector (Math|Random|RandomFloatinRange 0.0 (.x _spacing)) (Math|Random|RandomFloatinRange 0.0 (.y _spacing)) (Math|Random|RandomFloatinRange 0.0 (.z _spacing)))) _returnvalue_4 "2.000000,2.000000,2.000000") false)))))))