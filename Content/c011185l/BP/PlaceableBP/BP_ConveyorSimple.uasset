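; BP_ConveyorSimple is a placeable conveyor that pushes whatever sits inside its Box volume.
; Each Tick it offsets every overlapping actor's root along the Arrow's forward vector by Speed times delta seconds, without sweeping.
; An alternative BP_Box-only push and a timer-driven, endlessly increasing value are left disconnected, and the overlap events do nothing.
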(event OnComponentBeginOverlap(Box)
  (params (OverlappedComponent :type Primitive%20Component%20Object%20Reference) (OtherActor :type Actor%20Object%20Reference) (OtherComp :type Primitive%20Component%20Object%20Reference) (OtherBodyIndex :type Integer) (bFromSweep :type Boolean) (SweepResult :type Hit%20Result%20Structure%20%28by%20ref%29))
  ;[1 1 1] alertnate that just effects the box
)

(event OnComponentEndOverlap(Box)
  (params (OverlappedComponent :type Primitive%20Component%20Object%20Reference) (OtherActor :type Actor%20Object%20Reference) (OtherComp :type Primitive%20Component%20Object%20Reference) (OtherBodyIndex :type Integer))
  ;[1 1 1] alertnate that just effects the box
)

(event Custom|ApplyMovement
  ;[1 1 1] speeds up forever
  (Variables|Default|Setincreasing (+ (Variables|Default|Getincreasing) 0.001)))

(event EventTick
  (params (DeltaSeconds :type Float%20%28single-precision%29))
  (|CallParentFunction DeltaSeconds)
  (bind _output_get (Variables|Default|SetOverlapping%20Actors (Collision|GetOverlappingActors (Variables|Default|GetBox) 0 :!class /Script/Engine.PrimitiveComponent)))
  (for _array_element _output_get
    (Transformation|AddWorldOffset (Variables|/Script/Engine.Actor|GetRootComponent _array_element) (* (Math|Vector|GetForwardVector (Transformation|GetWorldRotation (Variables|Default|GetArrow))) (* DeltaSeconds (Variables|Default|Getspeed))) false false)))

(event EventBeginPlay
  (|CallParentFunction))

(fn ConstructionScript
  (|CallParentFunction))